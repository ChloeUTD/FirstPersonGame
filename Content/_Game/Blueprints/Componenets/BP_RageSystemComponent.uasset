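; Actor component that manages a rage resource, starting full and regenerating over time up to a maximum.
; A looping timer, rather than Tick, applies regeneration at a set frequency.
; Spend Rage deducts the cost only when affordable, then pauses regeneration for a set duration.
; Pausing schedules a resume timer for positive durations, and otherwise holds until Start Tick Rage is called.
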(event `self.ReceiveBeginPlay`
  ; Set rage to max
  (set `self.Rage` (`self.MaxRage`))
  ; Call Tick Rage
  (bind _returnvalue (`KismetSystemLibrary.K2_SetTimer` null "Tick Rage" (`self.RageTickFrequency`) true))
  (set `self.RageTickTimer` _returnvalue))

(fn `Pause Tick Rage`
  (params (Duration :type "Float (double-precision)"))
  (`KismetSystemLibrary.K2_PauseTimerHandle` (`self.RageTickTimer`))
  (if (> Duration 0.0)
    (`KismetSystemLibrary.K2_SetTimer` null "Start Tick Rage" Duration)))

(fn `Spend Rage`
  (if (<= (`self.RageCost`) (`self.Rage`))
    (set `self.Rage` (`KismetMathLibrary.FClamp` (- (`self.Rage`) (`self.RageCost`)) 0.0 (`self.Rage`)))
    (`self.Pause Tick Rage` (`self.RageSpendPauseDuration`))))

(fn `Start Tick Rage`
  (`KismetSystemLibrary.K2_UnPauseTimerHandle` (`self.RageTickTimer`)))

(fn `Tick Rage`
  (set `self.Rage` (`KismetMathLibrary.FClamp` (+ (`self.Rage`) (* (`self.RageRegenPerSecond`) (`self.RageTickFrequency`))) 0.0 (`self.MaxRage`))))