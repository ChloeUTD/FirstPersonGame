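; Actor component that manages a stamina pool, starting full and regenerating over time.
; A looping timer, rather than Tick, adds regen each interval, clamped to the maximum.
; SpendStamina deducts only affordable amounts, then pauses regen through PauseTickStamina, which uses a named timer to resume it after the delay.
; A non-positive pause duration leaves regen paused, and StopTickStamina is an empty stub.
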(event `self.ReceiveBeginPlay`
  ; Set stamina to max
  (set `self.Stamina` (`self.MaxStamina`))
  ; Calls tick stamina
  (bind _returnvalue (`KismetSystemLibrary.K2_SetTimer` null "Tick Stamina" (`self.StaminaTickFrequency`) true))
  (set `self.StaminaTickTimer` _returnvalue))

(fn `PauseTickStamina`
  (params (Duration :type "Float (double-precision)"))
  (`KismetSystemLibrary.K2_PauseTimerHandle` (`self.StaminaTickTimer`))
  (if (> Duration 0.0)
    (`KismetSystemLibrary.K2_SetTimer` null "Start Tick Stamina" Duration)))

(fn `Spend Stamina`
  (params (Amount :type "Float (double-precision)"))
  ; Checks if current stamina
  (if (<= Amount (`self.Stamina`))
    (set `self.Stamina` (`KismetMathLibrary.FClamp` (- (`self.Stamina`) Amount) 0.0 (`self.Stamina`)))
    (`self.PauseTickStamina` (`self.StaminaSpendPauseDuration`))))

(fn `Start Tick Stamina`
  (`KismetSystemLibrary.K2_UnPauseTimerHandle` (`self.StaminaTickTimer`)))

(fn `Stop Tick Stamina`)

(fn `Tick Stamina`
  (set `self.Stamina` (`KismetMathLibrary.FClamp` (+ (`self.Stamina`) (* (`self.StaminaRegenPerSec`) (`self.StaminaTickFrequency`))) 0.0 (`self.MaxStamina`))))