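; An exploding barrel that, when its health component reports it killed, damages nearby actors that have a health component.
; Targets come from a sphere overlap with itself removed, and each hit also plays a camera shake centred on the player.
; A BeenKilled flag, set after the damage loop, is meant to prevent repeat explosions.
; It hides the mesh, disables collision, spawns effect and sound, then destroys itself when the sound ends.
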(event `self.ReceiveBeginPlay`
  (add `/Game/_Game/Blueprints/Componenets/BP_HealthSystemComponent.OnKilled` (`self.BP_HealthSystemComponent`) (delegate `OnKilled`)))

(event `OnKilled`
  (bind _sound (`self.Sound`))
  (if (not (`self.BeenKilled`))
    ; removes self from list (DO NOT REMOVE IT WILL MAKE AN INFINITE LOOP)
    (bind _output_get (set `self.Overlapping Actors` (`PrimitiveComponent.GetOverlappingActors` (`self.Sphere`) null)))
    (`KismetArrayLibrary.Array_RemoveItem` _output_get self)
    ; Gets every actor but self and deals damage to them
    (for _array_element (`self.Overlapping Actors`)
      (bind _returnvalue (`self.GetComponentByClass` _array_element "/Game/_Game/Blueprints/Componenets/BP_HealthSystemComponent.BP_HealthSystemComponent_C"))
      (`/Engine/EditorBlueprintResources/StandardMacros.IsValid` _returnvalue ; If the component has health system its added to list
        (:`Is Valid`
          (`/Game/_Game/Blueprints/Componenets/BP_HealthSystemComponent.TookDamage` _returnvalue _array_element (`self.Damage`) null null null)
          (`GameplayStatics.PlayWorldCameraShake` "/Game/_Game/Blueprints/BP_CamShake.BP_CamShake_C" (`self.K2_GetActorLocation` (`GameplayStatics.GetPlayerCharacter` 0)) 0.0 2000.0))))
    (set `self.BeenKilled` true)
    (`SceneComponent.SetVisibility` (`self.Cylinder`) false false)
    (`PrimitiveComponent.SetCollisionEnabled` (`self.Cylinder`) "NoCollision") ; Fixes gunshots hitting invisible barrel
    (`NiagaraFunctionLibrary.SpawnSystemAtLocation` "/Game/Particles1/PS_Explosion.PS_Explosion" (`self.K2_GetActorLocation` self))
    (`GameplayStatics.PlaySoundAtLocation` _sound (`self.K2_GetActorLocation` self) (struct) 1.0 1.0 0.0 null null null null)
    (`KismetSystemLibrary.Delay` (`SoundBase.Duration` _sound))
    (`self.K2_DestroyActor`) ; Doesn't fix infinite loop
  ))

(fn `UserConstructionScript`)